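; Widget component for enemies, named as a combat preview, that drives its material from the owning enemy's faction and a kill flag.
; One second after BeginPlay, it casts its owner to BP_BaseEnemy, sets the "Type" parameter by whether the faction is the first enum value, then enables updates.
; Each tick after that, it copies CanKill into the "canKill" material parameter, polling rather than reacting to changes.
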(event `self.ReceiveBeginPlay`
  (`KismetSystemLibrary.Delay` 1.0)
  (bind _asbp_base_enemy (cast `/Game/Blueprints/Enemies/BP_BaseEnemy` (`self.GetOwner`)))
  (`MaterialInstanceDynamic.SetScalarParameterValue` (`self.GetMaterialInstance`) "Type" (`KismetMathLibrary.Conv_BoolToDouble` (== (`GridEnemyPawn.Faction` _asbp_base_enemy) 0)))
  (set `self.enableTick` true))

(event `self.ReceiveTick`
  (params (DeltaSeconds :type "Float (single-precision)"))
  (if (`self.enableTick`)
    (`MaterialInstanceDynamic.SetScalarParameterValue` (`self.GetMaterialInstance`) "canKill" (`KismetMathLibrary.Conv_BoolToDouble` (`self.canKill`)))))