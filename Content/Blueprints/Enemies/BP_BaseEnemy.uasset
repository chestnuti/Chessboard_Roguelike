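; BP_BaseEnemy is the base Blueprint for grid enemies, adding visual feedback for ranged attacks and death.
; BeginPlay gives the ranged telegraph a dynamic material tinted by faction flag and binds fragment spawning to the grid-enemy-killed event.
; Aim start feeds the pending grid direction to that material, yaws the mesh and caches the direction.
; Attack resolution shakes the camera and launches a short-lived Niagara VFX actor along it.
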(event `self.ReceiveTick`
  (params (DeltaSeconds :type "Float (single-precision)")))

(event `self.ReceiveBeginPlay`
  (bind _rangedattacktelegraphcomponent (`self.RangedAttackTelegraphComponent`))
  (`|ExecutionSequence`
    (:`then_0`
      ; set ranged attack range material
      (bind _returnvalue (`KismetMaterialLibrary.CreateDynamicMaterialInstance` (`RangedAttackTelegraphComponent.TelegraphMaterial` _rangedattacktelegraphcomponent)))
      (bind _output_get (set `self.AttackRange_MID` _returnvalue))
      (set `RangedAttackTelegraphComponent.TelegraphMaterial` _output_get _rangedattacktelegraphcomponent)
      (`MaterialInstanceDynamic.SetScalarParameterValue` (`self.AttackRange_MID`) "Faction" (`KismetMathLibrary.Conv_BoolToDouble` (== (`self.Faction`) 0))))
    (:`then_1`
      (add `self.OnGridEnemyKilled` (delegate `SpawnFragments`)))))

(event `SpawnFragments` :!signature `self.OnGridEnemyKilled`
  (params (Enemy :type "GridEnemyPawn Object Reference") (DeathCoord :type "IntPoint Structure") (DeathWorldLocation :type "Vector Structure"))
  (bind _fragmentsactor (`self.FragmentsActor`))
  ; Spawn Death Fragments
  (if (`KismetSystemLibrary.IsValidClass` _fragmentsactor)
    (bind _returnvalue (`|SpawnActorFromClass` _fragmentsactor (`KismetMathLibrary.MakeTransform` DeathWorldLocation) "Undefined" "MultiplyWithRoot" null null))
    (`KismetSystemLibrary.Delay` 3.0)
    (`self.K2_DestroyActor` _returnvalue)))

(event `self.OnRangedAimStarted`
  (params (PlayerPawn :type "GridPawn Object Reference") (AttackTiles :type "Array of IntPoint Structure (by ref)"))
  (bind _attackrange_mid (`self.AttackRange_MID`))
  (bind (_x _y) (break `IntPoint` (`self.PendingRangedAttackDirection`)))
  (bind (_x_2 _y_2) (break `IntPoint` (`self.PendingRangedAttackDirection`)))
  (bind (_x_3 _y_3) (break `IntPoint` (`self.PendingRangedAttackDirection`)))
  (`|ExecutionSequence`
    (:`then_0`
      ; Set ranged attack direction
      (`/Engine/EditorBlueprintResources/StandardMacros.IsValid` _attackrange_mid
        (:`Is Valid`
          (`MaterialInstanceDynamic.SetScalarParameterValue` _attackrange_mid "DirectionX" (`KismetMathLibrary.Conv_IntToDouble` _x_2))
          (`MaterialInstanceDynamic.SetScalarParameterValue` _attackrange_mid "DirectionY" (`KismetMathLibrary.Conv_IntToDouble` _y_2)))))
    (:`then_1`
      ; Rotate to Aim
      (`SceneComponent.K2_SetRelativeRotation` (`self.EnemyMesh`) (`KismetMathLibrary.MakeRotator` 0.0 0.0 (`KismetMathLibrary.Conv_IntToDouble` (+ (* _x_3 -90) (* (+ (* _y_3 -90) 90) (`KismetMathLibrary.Abs_Int` _y_3))))) false false)
      ; Save Attack Direction
      (set `self.AttackDirection` (`KismetMathLibrary.MakeVector` (`KismetMathLibrary.Conv_IntToDouble` _x) (`KismetMathLibrary.Conv_IntToDouble` _y))))))

(event `self.OnRangedAttackResolved`
  (params (PlayerPawn :type "GridPawn Object Reference") (AttackTiles :type "Array of IntPoint Structure (by ref)") (AttackResult :type "EnemyAttackResolveResult Structure") (bHitPlayer :type Boolean))
  ; Camera Shake on ranged attack
  (`PlayerController.ClientStartCameraShake` :`self` (`GameplayStatics.GetPlayerController` 0) :`Shake` "/Game/Blueprints/CameraShake/BPCS_RangedAttack.BPCS_RangedAttack_C" :`Scale` 0.05)
  ; Attack VFX
  (bind _returnvalue (`|SpawnActorFromClass` "/Game/Blueprints/Enemies/VFX/BP_RangedAttackVFX.BP_RangedAttackVFX_C" (`KismetMathLibrary.MakeTransform` (`SceneComponent.K2_GetComponentLocation` (`self.EnemyMesh`))) "Undefined" "MultiplyWithRoot" null null))
  (set `/Game/Blueprints/Enemies/VFX/BP_RangedAttackVFX.Direction` (`self.AttackDirection`) _returnvalue)
  (set `/Game/Blueprints/Enemies/VFX/BP_RangedAttackVFX.Speed` 10000.0 _returnvalue)
  (set `/Game/Blueprints/Enemies/VFX/BP_RangedAttackVFX.Niagara` (`self.RangedNiagara`) _returnvalue)
  (`KismetSystemLibrary.Delay` 2.0)
  (`self.K2_DestroyActor` _returnvalue))

(fn `UserConstructionScript`)