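; BP_GridManager is a grid actor that plays a build-in animation on the materials of its TileISM component.
; BeginPlay resets the BuildDistance material parameter, then enables the build after a short delay.
; Tick then raises BuildDistance at BuildSpeed up to a fixed limit and pushes it to the materials, leaving the visual effect to the shader.
; No tile creation or grid logic appears in these graphs.
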(event `self.ReceiveBeginPlay`
  ; Ready for Grid build
  (`MeshComponent.SetScalarParameterValueOnMaterials` (`self.TileISM`) "BuildDistance" 0.0)
  (`KismetSystemLibrary.Delay` 1.0)
  (set `self.enableBuild` true))

(event `self.ReceiveTick`
  (params (DeltaSeconds :type "Float (single-precision)"))
  (if (`self.enableBuild`)
    ; Gird Build Animation
    (`/Engine/EditorBlueprintResources/StandardMacros.CompareFloat` (`self.BuildDistance`) 1000.0
      (:`<`
        (bind _output_get (set `self.BuildDistance` (+ (`self.BuildDistance`) (* DeltaSeconds (`self.BuildSpeed`)))))
        (`MeshComponent.SetScalarParameterValueOnMaterials` (`self.TileISM`) "BuildDistance" _output_get)))))

(fn `UserConstructionScript`)