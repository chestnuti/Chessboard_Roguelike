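; Player component on GridPawn that drives EnergyMesh, a spinning indicator of the held conversion energy.
; It binds to the ConversionEnergyComponent's granted and consumed events to show, or hide after a short delay, the mesh through material parameters.
; Gain, use and switch spike a glow strength that lerps back each tick, with gain and switch also updating the type parameter.
; Use-energy input toggles a material shake and ramps its speed while ongoing.
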(event `EnergyGranted`
  (params (EnergyType :type "ETileType Enum" :default "Minimal"))
  (bind _energymesh (`self.EnergyMesh`))
  ; Show energy indicate mesh when gain
  (`MeshComponent.SetScalarParameterValueOnMaterials` _energymesh "hasEnergy" 1.0)
  (`MeshComponent.SetScalarParameterValueOnMaterials` _energymesh "EnergyType" (`KismetMathLibrary.Conv_BoolToDouble` (== (`ConversionEnergyComponent.GetHeldConversionEnergyType` (`self.Conversion Energy Component`)) 1)))
  (set `self.TwinkleValue` 50.0))

(event `self.ReceiveBeginPlay`
  (bind _asgrid_pawn (cast `GridPawn` (`self.GetOwner`)))
  (bind _output_get (set `self.As Grid Pawn` _asgrid_pawn))
  (set `self.Conversion Energy Component` (`GridPawn.ConversionEnergyComponent` _output_get))
  (`|ExecutionSequence`
    (:`then_0`
      ; Show energy indicate mesh when gain
      (add `ConversionEnergyComponent.OnConversionEnergyGranted` (`self.Conversion Energy Component`) (delegate `EnergyGranted`)))
    (:`then_1`
      ; Hide energy indicate mesh after used
      (add `ConversionEnergyComponent.OnConversionEnergyConsumed` (`self.Conversion Energy Component`) (delegate `EnergyConsumed`)))))

(event `EnergyConsumed`
  (params (EnergyType :type "ETileType Enum" :default "Minimal"))
  ; Hide energy indicate mesh after used
  (set `self.TwinkleValue` 50.0)
  (`KismetSystemLibrary.Delay` 0.3)
  (`MeshComponent.SetScalarParameterValueOnMaterials` (`self.EnergyMesh`) "hasEnergy" 0.0))

(event `self.ReceiveTick`
  (params (DeltaSeconds :type "Float (single-precision)"))
  (`|ExecutionSequence`
    (:`then_0`
      (`SceneComponent.K2_AddLocalRotation` (`self.EnergyMesh`) (struct :`Yaw` 1.0) false false))
    (:`then_1`
      ; Twinkle
      (if true
        (bind _output_get (set `self.TwinkleValue` (`KismetMathLibrary.Lerp` (`self.TwinkleValue`) 1.0 0.2)))
        (`MeshComponent.SetScalarParameterValueOnMaterials` (`self.EnergyMesh`) "Strength" _output_get)))))

(event `EnhancedInput|/Game/Data/Input/IA_SwitchEnergy`
  (params (ActionValue :type Boolean) (ElapsedSeconds :type "Float (double-precision)") (TriggeredSeconds :type "Float (double-precision)") (InputAction :type "InputAction Object Reference" :default "/Game/Data/Input/IA_SwitchEnergy.IA_SwitchEnergy"))
  (:`Triggered`
    ; Energy switch
    (`MeshComponent.SetScalarParameterValueOnMaterials` (`self.EnergyMesh`) "EnergyType" (`KismetMathLibrary.Conv_BoolToDouble` (== (`ConversionEnergyComponent.GetHeldConversionEnergyType` (`self.Conversion Energy Component`)) 1)))
    (set `self.TwinkleValue` 50.0)))

(event `EnhancedInput|/Game/Data/Input/IA_UseEnergy`
  (params (ActionValue :type Boolean) (ElapsedSeconds :type "Float (double-precision)") (TriggeredSeconds :type "Float (double-precision)") (InputAction :type "InputAction Object Reference" :default "/Game/Data/Input/IA_UseEnergy.IA_UseEnergy"))
  (bind _energymesh (`self.EnergyMesh`))
  (:`Triggered`
    ; Using Energy shake
    (`MeshComponent.SetScalarParameterValueOnMaterials` _energymesh "Shake" 1.0 :!label _label)
    (set `self.ShakeSpeed` 0.0 :!label _label_2))
  (:`Started`
    (goto _label))
  (:`Ongoing`
    (bind _output_get (set `self.ShakeSpeed` (`KismetMathLibrary.Lerp` (`self.ShakeSpeed`) 0.1 0.1)))
    (`MeshComponent.SetScalarParameterValueOnMaterials` _energymesh "ShakeSpeed" _output_get))
  (:`Canceled`
    (`MeshComponent.SetScalarParameterValueOnMaterials` _energymesh "Shake" 0.0 :!label _label_3)
    (goto _label_2))
  (:`Completed`
    (goto _label_3)))