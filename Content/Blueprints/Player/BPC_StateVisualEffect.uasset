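; Player pawn component that drives visual feedback for conversion energy, transformation, maxed attributes and health changes.
; BeginPlay binds to the pawn's energy, attribute and transform events, which spawn transform VFX, toggle fire effects and write to mesh materials and MPC_PlayerState.
; Tick spins the energy mesh and eases event-spiked twinkle and hurt/heal values back to rest.
; Energy input adds shake and charge audio, while damage triggers camera shake and time-dilation hit stop.
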(event `EnergyGranted`
  (params (EnergyType :type "ETileType Enum" :default "Minimal"))
  (bind _energymesh (`self.EnergyMesh`))
  ; Show energy indicate mesh when gain
  (`MeshComponent.SetScalarParameterValueOnMaterials` _energymesh "hasEnergy" 1.0)
  (`MeshComponent.SetScalarParameterValueOnMaterials` _energymesh "EnergyType" (`KismetMathLibrary.Conv_BoolToDouble` (== (`ConversionEnergyComponent.GetHeldConversionEnergyType` (`self.Conversion Energy Component`)) 1)))
  (set `self.EnergyTwinkleValue` 50.0))

(event `self.ReceiveBeginPlay`
  (bind _asbp_grid_pawn (cast `/Game/Blueprints/Player/BP_GridPawn` (`self.GetOwner`)))
  (bind _output_get (set `self.As Grid Pawn` _asbp_grid_pawn))
  (set `self.Conversion Energy Component` (`GridPawn.ConversionEnergyComponent` _output_get))
  (`|ExecutionSequence`
    (:`then_0`
      ; Show energy indicate mesh when gain
      (add `ConversionEnergyComponent.OnConversionEnergyGranted` (`self.Conversion Energy Component`) (delegate `EnergyGranted`)))
    (:`then_1`
      ; Hide energy indicate mesh after used or dead
      (add `ConversionEnergyComponent.OnConversionEnergyConsumed` (`self.Conversion Energy Component`) (delegate `EnergyConsumed`))
      (add `PlayerAttributeComponent.OnPlayerDefeated` (`GridPawn.PlayerAttributeComponent` (`self.As Grid Pawn`)) (delegate `PlayerDead`)))
    (:`then_2`
      ; Player Transform VFX
      (add `GridPawn.OnTransformVisualStateChanged` (`self.As Grid Pawn`) (delegate `PawnChanged`)))
    (:`then_3`
      ; Check if attribute max
      (add `PlayerAttributeComponent.OnPlayerAttributeChanged` (`GridPawn.PlayerAttributeComponent` (`self.As Grid Pawn`)) (delegate `isAttributeMax`)))
    (:`then_4`
      ; Player HP Change
      (add `PlayerAttributeComponent.OnPlayerHealthChanged` (`GridPawn.PlayerAttributeComponent` (`self.As Grid Pawn`)) (delegate `HealthChanged`)))))

(event `EnergyConsumed`
  (params (EnergyType :type "ETileType Enum" :default "Minimal"))
  ; Hide energy indicate mesh after used or dead
  (set `self.EnergyTwinkleValue` 50.0 :!label _label)
  (`KismetSystemLibrary.Delay` 0.3)
  (`MeshComponent.SetScalarParameterValueOnMaterials` (`self.EnergyMesh`) "hasEnergy" 0.0))

(event `PlayerDead`
  ; Hide energy indicate mesh after used or dead
  (goto _label))

(event `PawnChanged`
  (params (FormData :type "ChessPieceFormData Object Reference") (bIsTransformed :type Boolean))
  (bind _returnvalue (`KismetMathLibrary.MakeTransform` (`SceneComponent.K2_GetComponentLocation` (`GridPawn.PawnMesh` (`self.As Grid Pawn`)))))
  ; Player Transform VFX
  (bind _returnvalue_2 (`|SpawnActorFromClass` "/Game/Characters/Player/VFX/BP_TransfromVFX.BP_TransfromVFX_C" _returnvalue "Undefined" "MultiplyWithRoot" null null))
  (`|ExecutionSequence`
    (:`then_0`
      (if bIsTransformed
        (bind _returnvalue_3 (`|SpawnActorFromClass` "/Game/Characters/Player/VFX/BP_KeepTransfrom.BP_KeepTransfrom_C" _returnvalue "Undefined" "MultiplyWithRoot" null null))
        (set `self.TransformingVFX` _returnvalue_3)
        (else
          (`Actor.K2_DestroyActor` (`self.TransformingVFX`)))))
    (:`then_1`
      (`KismetSystemLibrary.Delay` 2.0)
      (`Actor.K2_DestroyActor` _returnvalue_2))))

(event `EnhancedInput|/Game/Data/Input/IA_SwitchEnergy`
  (params (ActionValue :type Boolean) (ElapsedSeconds :type "Float (double-precision)") (TriggeredSeconds :type "Float (double-precision)") (InputAction :type "InputAction Object Reference" :default "/Game/Data/Input/IA_SwitchEnergy.IA_SwitchEnergy"))
  (:`Triggered`
    ; Energy switch
    (`MeshComponent.SetScalarParameterValueOnMaterials` (`self.EnergyMesh`) "EnergyType" (`KismetMathLibrary.Conv_BoolToDouble` (== (`ConversionEnergyComponent.GetHeldConversionEnergyType` (`self.Conversion Energy Component`)) 1)))
    (set `self.EnergyTwinkleValue` 50.0)))

(event `self.ReceiveTick`
  (params (DeltaSeconds :type "Float (single-precision)"))
  (`|ExecutionSequence`
    (:`then_0`
      (`SceneComponent.K2_AddLocalRotation` (`self.EnergyMesh`) (struct :`Yaw` 1.0) false false))
    (:`then_1`
      ; Energy Twinkle
      (if true
        (bind _output_get (set `self.EnergyTwinkleValue` (`KismetMathLibrary.Lerp` (`self.EnergyTwinkleValue`) 1.0 (* DeltaSeconds 10.0))))
        (`MeshComponent.SetScalarParameterValueOnMaterials` (`self.EnergyMesh`) "Strength" _output_get)))
    (:`then_2`
      ; Player Twinkle
      (bind _output_get_2 (set `self.PlayerTwinkleValue` (`KismetMathLibrary.Lerp` (`self.PlayerTwinkleValue`) 0.0 (* DeltaSeconds 10.0))))
      (`MeshComponent.SetScalarParameterValueOnMaterials` (`GridPawn.PawnMesh` (`self.As Grid Pawn`)) "Strength" _output_get_2))
    (:`then_3`
      ; Player HP Change
      (bind _output_get_3 (set `self.HurtOrHeal` (`KismetMathLibrary.Lerp` (`self.HurtOrHeal`) 0.0 (* DeltaSeconds 2.0))))
      (`MeshComponent.SetScalarParameterValueOnMaterials` (`GridPawn.PawnMesh` (`self.As Grid Pawn`)) "HurtOrHeal" _output_get_3))))

(event `EnhancedInput|/Game/Data/Input/IA_UseEnergy`
  (params (ActionValue :type Boolean) (ElapsedSeconds :type "Float (double-precision)") (TriggeredSeconds :type "Float (double-precision)") (InputAction :type "InputAction Object Reference" :default "/Game/Data/Input/IA_UseEnergy.IA_UseEnergy"))
  (bind _returnvalue (`GameAudioBlueprintLibrary.GetGameAudioSubsystem`))
  (bind _energymesh (`self.EnergyMesh`))
  (:`Triggered`
    ; Using Energy shake
    (`MeshComponent.SetScalarParameterValueOnMaterials` _energymesh "Shake" 1.0 :!label _label_2)
    (set `self.ShakeSpeed` 0.0 :!label _label_3)
    (`GameAudioSubsystem.StopPlayerPrepareUseEnergySFX` _returnvalue 0.0))
  (:`Started`
    (goto _label_2))
  (:`Ongoing`
    (bind _output_get (set `self.ShakeSpeed` (`KismetMathLibrary.Lerp` (`self.ShakeSpeed`) 0.1 0.1)))
    (`MeshComponent.SetScalarParameterValueOnMaterials` _energymesh "ShakeSpeed" _output_get)
    (`GameAudioSubsystem.StartPlayerPrepareUseEnergySFX` _returnvalue 0.0 false))
  (:`Canceled`
    (`MeshComponent.SetScalarParameterValueOnMaterials` _energymesh "Shake" 0.0 :!label _label_4)
    (goto _label_3))
  (:`Completed`
    (goto _label_4)))

(event `isAttributeMax`
  (params (NewConstructValue :type Integer) (NewAcidValue :type Integer))
  (bind _returnvalue (== NewConstructValue 10))
  (bind _returnvalue_2 (== NewAcidValue 10))
  (bind _as_grid_pawn (`self.As Grid Pawn`))
  (bind _returnvalue_3 (or _returnvalue _returnvalue_2))
  ; Check if attribute max
  (`KismetSystemLibrary.Delay` 0.2)
  (`|ExecutionSequence`
    (:`then_0`
      (`KismetMaterialLibrary.SetScalarParameterValue` "/Game/Materials/MPC/MPC_PlayerState.MPC_PlayerState" "MaxType" (`KismetMathLibrary.Conv_IntToDouble` (- (`KismetMathLibrary.SelectInt` 1 0 _returnvalue) (not _returnvalue_3))))
      (if _returnvalue_3
        (set `self.PlayerTwinkleValue` 200.0)
        (bind _returnvalue_4 (`|SpawnActorFromClass` "/Game/Characters/Player/VFX/BP_TransfromVFX.BP_TransfromVFX_C" (`KismetMathLibrary.MakeTransform` (`SceneComponent.K2_GetComponentLocation` (`GridPawn.PawnMesh` (`self.As Grid Pawn`)))) "Undefined" "MultiplyWithRoot" null null))
        (`KismetSystemLibrary.Delay` 2.0)
        (`Actor.K2_DestroyActor` _returnvalue_4)))
    (:`then_1`
      (`SceneComponent.SetVisibility` (`/Game/Blueprints/Player/BP_GridPawn.NS_Construct_Fire` _as_grid_pawn) _returnvalue false))
    (:`then_2`
      (`SceneComponent.SetVisibility` (`/Game/Blueprints/Player/BP_GridPawn.NS_Acid_Fire` _as_grid_pawn) _returnvalue_2 false))))

(event `HealthChanged`
  (params (NewHealth :type Integer) (MaxHealth :type Integer))
  (bind _returnvalue (- NewHealth (`self.CurrentHP`)))
  ; Player HP Change
  (`/Engine/EditorBlueprintResources/StandardMacros.CompareFloat` _returnvalue
    (:`>`
      (set `self.HurtOrHeal` _returnvalue :!label _label_5)
      (set `self.CurrentHP` (`KismetMathLibrary.Conv_IntToDouble` NewHealth))
      (set `self.PlayerTwinkleValue` 50.0)
      (`KismetMaterialLibrary.SetScalarParameterValue` "/Game/Materials/MPC/MPC_PlayerState.MPC_PlayerState" "HP" (`KismetMathLibrary.Conv_IntToDouble` NewHealth)))
    (:`==`
      (goto _label_5))
    (:`<`
      (`|ExecutionSequence`
        (:`then_0`
          (goto _label_5))
        (:`then_1`
          ; HitStop
          (`KismetSystemLibrary.Delay` 0.1)
          (`PlayerController.ClientStartCameraShake` :`self` (`GameplayStatics.GetPlayerController` 0) :`Shake` "/Game/Blueprints/CameraShake/BPCS_KillEnemy.BPCS_KillEnemy_C" :`Scale` 0.05)
          (`GameplayStatics.SetGlobalTimeDilation` 0.1)
          (`KismetSystemLibrary.Delay` 0.015)
          (`GameplayStatics.SetGlobalTimeDilation` 1.0))))))