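; Player controller for the grid dungeon that runs screen-mask fade transitions between levels.
; BeginPlay creates the mask widget, starts revealing the screen, and binds dungeon level and tutorial completion events to trigger a fade to masked.
; Tick eases the material's Mask parameter with a fixed-alpha, frame-rate-dependent Lerp.
; Once masked, it waits briefly, tells BP_DungeonRunManager to advance to the next level, then fades back out.
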(event `self.ReceiveBeginPlay`
  (`parent.ReceiveBeginPlay`)
  ; Start Fade out
  (`|ExecutionSequence`
    (:`then_0`
      (bind _returnvalue (`|CreateWidget` "/Game/UI/WBP_ScreenMaskTransition.WBP_ScreenMaskTransition_C"))
      (`UserWidget.AddToViewport` _returnvalue 1)
      (bind _returnvalue_2 (`Image.GetDynamicMaterial` (`/Game/UI/WBP_ScreenMaskTransition.Image_0` _returnvalue)))
      (`MaterialInstanceDynamic.SetScalarParameterValue` _returnvalue_2 "Mask" 1.0)
      (set `self.FadeOut` true))
    (:`then_1`
      (bind _returnvalue_3 (`GameplayStatics.GetActorOfClass` "/Game/Blueprints/Grid/BP_DungeonRunManager.BP_DungeonRunManager_C"))
      (add `DungeonRunManager.OnDungeonLevelCompleted` _returnvalue_3 (delegate `DungeonLevelCompleted`))
      (add `TutorialFlowComponent.OnTutorialFlowCompleted` (`self.TutorialFlowComponent`) (delegate `TutorialFlowCompleted`)))))

(event `TutorialFlowCompleted`
  (params (CompletedFlow :type "TutorialFlowDataAsset Object Reference"))
  ; Start Fade out
  (set `self.FadeIn` true :!label _label))

(event `DungeonLevelCompleted`
  (params (CompletedLevelIndex :type Integer) (NextLevelIndex :type Integer))
  ; Start Fade out
  (goto _label))

(event `self.ReceiveTick`
  (params (DeltaSeconds :type "Float (single-precision)"))
  (`parent.ReceiveTick` DeltaSeconds)
  ; Fading Anime
  (`|ExecutionSequence`
    (:`then_0`
      (if (`self.FadeIn`)
        (bind _image_0 (`/Game/UI/WBP_ScreenMaskTransition.Image_0` (stale `self.ReceiveBeginPlay` _returnvalue)))
        (bind _completed (`self.ScreenTransition` _image_0 1.0))
        (if _completed
          (set `self.FadeIn` false)
          (`self.NextLevel`))))
    (:`then_1`
      (if (`self.FadeOut`)
        (bind _completed_2 (`self.ScreenTransition` _image_0))
        (if _completed_2
          (set `self.FadeOut` false))))))

(event `NextLevel`
  ; Next Level
  (`KismetSystemLibrary.Delay` 1.0)
  (bind _returnvalue (`GameplayStatics.GetActorOfClass` "/Game/Blueprints/Grid/BP_DungeonRunManager.BP_DungeonRunManager_C"))
  (`DungeonRunManager.AdvanceToNextLevel` _returnvalue)
  (set `self.FadeOut` true))

(fn `ScreenTransition`
  (params (`Dynamic Material` :type "Image Object Reference") (AimValue :type "Float (double-precision)"))
  (returns (Completed :type Boolean))
  (bind _returnvalue (`Image.GetDynamicMaterial` `Dynamic Material`))
  (bind _output_get (set `self.FadeValue` (`KismetMathLibrary.Lerp` (`self.FadeValue`) AimValue 0.1)))
  (`MaterialInstanceDynamic.SetScalarParameterValue` _returnvalue "Mask" _output_get)
  (return (<= (`KismetMathLibrary.Abs` (- (`self.FadeValue`) AimValue)) 0.1)))

(fn `UserConstructionScript`
  (`parent.UserConstructionScript`))