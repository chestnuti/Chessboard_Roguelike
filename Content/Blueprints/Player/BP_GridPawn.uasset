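; BP_GridPawn is the player's grid-based pawn, which earns conversion energy by killing enemies and spends it to convert surrounding tiles.
; Kills set HasEnergy and play hit-stop through the pawn's CustomTimeDilation with a camera shake.
; Enhanced Input toggles Acid or Construct energy and triggers ConvertAreaAroundPlayer on the grid manager, consuming the charge.
; Tick prints current tile debug data, and a helper lerps spring-arm length for zoom.
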(event `self.ReceiveTick`
  (params (DeltaSeconds :type "Float (single-precision)"))
  (bind _currentgridcoord (`self.CurrentGridCoord`))
  (`parent.ReceiveTick` DeltaSeconds)
  (`|ExecutionSequence`
    (:`then_1`
      (bind _returnvalue (`GameplayStatics.GetActorOfClass` "/Game/Blueprints/Grid/BP_GridManager.BP_GridManager_C"))
      (bind (_gridcoord _tiletype _cellrole _regionid _depth) (break `TileData` (`GridManager.GetTileData` _returnvalue _currentgridcoord)))
      (`KismetSystemLibrary.PrintString` (`KismetStringLibrary.Concat_StrStr` (`KismetStringLibrary.Concat_StrStr` (`KismetStringLibrary.Conv_IntPointToString` _currentgridcoord) (`KismetStringLibrary.Concat_StrStr` " Depth: " (`KismetStringLibrary.Conv_IntToString` _depth))) (`KismetStringLibrary.Concat_StrStr` " Cell: " (`|GetEnumeratorNameAsString` _cellrole)))))))

(event `self.OnPlayerKilledEnemy`
  (params (KilledEnemy :type "GridEnemyPawn Object Reference") (DroppedEnergyType :type "ETileType Enum" :default "Minimal"))
  (set `self.hasEnergy` true)
  ; HitStop
  (`KismetSystemLibrary.Delay` 0.11)
  (`PlayerController.ClientStartCameraShake` :`self` (`GameplayStatics.GetPlayerController` 0) :`Shake` "/Game/Blueprints/CameraShake/BPCS_KillEnemy.BPCS_KillEnemy_C" :`Scale` 0.05)
  (set `self.CustomTimeDilation` 0.05)
  (`KismetSystemLibrary.Delay` 0.3)
  (set `self.CustomTimeDilation` 1.0))

(event `EnhancedInput|/Game/Data/Input/IA_UseEnergy`
  (params (ActionValue :type Boolean) (ElapsedSeconds :type "Float (double-precision)") (TriggeredSeconds :type "Float (double-precision)") (InputAction :type "InputAction Object Reference" :default "/Game/Data/Input/IA_UseEnergy.IA_UseEnergy"))
  (:`Triggered`
    (`self.TryUseConversionEnergy`)
    (`KismetSystemLibrary.PrintString` "used energy")))

(event `EnhancedInput|/Game/Data/Input/IA_SwitchEnergy`
  (params (ActionValue :type Boolean) (ElapsedSeconds :type "Float (double-precision)") (TriggeredSeconds :type "Float (double-precision)") (InputAction :type "InputAction Object Reference" :default "/Game/Data/Input/IA_SwitchEnergy.IA_SwitchEnergy"))
  (:`Triggered`
    (bind _switchedtype (`self.SwitchUserConversionEnergy`))
    (`KismetSystemLibrary.PrintString` (`|GetEnumeratorNameAsString` _switchedtype))))

(fn `CameraZoomIn`
  (params (Speed :type "Float (double-precision)") (AimLength :type "Float (double-precision)"))
  (set `SpringArmComponent.TargetArmLength` (`KismetMathLibrary.Lerp` (`SpringArmComponent.TargetArmLength` (`self.SpringArm`)) AimLength Speed) (`self.SpringArm`)))

(fn `SwitchUserConversionEnergy`
  (returns (SwitchedType :type "ETileType Enum"))
  (locals (Acid :type "ETileType Enum" :default "Acid"))
  (bind _output_get (set `self.EnergyType` (select `bool` (== (`self.EnergyType`) (`local.Acid`)) :`false` "Acid" :`true` "Construct" :!type "ETileType Enum")))
  (return _output_get))

(fn `TryUseConversionEnergy`
  (if (`self.hasEnergy`)
    (bind _returnvalue (`GameplayStatics.GetActorOfClass` "/Script/Chessboard_Roguelike.GridManager"))
    (`self.ConvertAreaAroundPlayer` _returnvalue (`self.EnergyType`))
    (if true
      (set `self.hasEnergy` false))))

(fn `UserConstructionScript`
  (`parent.UserConstructionScript`))